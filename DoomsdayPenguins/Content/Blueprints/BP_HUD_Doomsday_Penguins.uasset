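; BP_HUD_Doomsday_Penguins manages the on-screen UI and mouse cursor for the penguin game, following state flags on BP_Penguin.
; On BeginPlay it clears the penguin's HasGameStarted flag, shows the WT_Doomsday_Penguin widget and enables the cursor.
; Tick polls the penguin, showing WT_In_Level_Quit with cursor on GameOver, or Gameplay without cursor once started.
; It creates and adds a new widget every frame while either state holds.
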(event EventBeginPlay
  (bind _returnvalue (Actor|GetActorOfClass "/Game/Blueprints/BP_Penguin.BP_Penguin_C"))
  (Variables|/Script/DoomsdayPenguins.Penguin|SetbHasGameStarted _returnvalue false)
  (bind _returnvalue_2 (UserInterface|CreateWidget "/Game/Blueprints/WT_Doomsday_Penguin.WT_Doomsday_Penguin_C" (Game|GetPlayerController 0)))
  (UserInterface|Viewport|AddtoViewport _returnvalue_2 0)
  (Variables|/Script/Engine.PlayerController|SetbShowMouseCursor (Game|GetPlayerController 0) true))

(event Collision|EventActorBeginOverlap
  (params (OtherActor :type Actor%20Object%20Reference)))

(event EventTick
  (params (DeltaSeconds :type Float%20%28single-precision%29))
  (bind _returnvalue (Actor|GetActorOfClass "/Game/Blueprints/BP_Penguin.BP_Penguin_C"))
  (if (Variables|/Script/DoomsdayPenguins.Penguin|GetGameOver _returnvalue)
    (bind _returnvalue_2 (UserInterface|CreateWidget "/Game/Blueprints/WT_In_Level_Quit.WT_In_Level_Quit_C" (Game|GetPlayerController 0)))
    (UserInterface|Viewport|AddtoViewport _returnvalue_2 0)
    (Variables|/Script/Engine.PlayerController|SetbShowMouseCursor (Game|GetPlayerController 0) true)
    (else
      (bind _returnvalue_3 (Actor|GetActorOfClass "/Game/Blueprints/BP_Penguin.BP_Penguin_C"))
      (if (Variables|/Script/DoomsdayPenguins.Penguin|GetbHasGameStarted _returnvalue_3)
        (bind _returnvalue_4 (UserInterface|CreateWidget "/Game/Blueprints/Gameplay.Gameplay_C"))
        (UserInterface|Viewport|AddtoViewport _returnvalue_4 0)
        (Variables|/Script/Engine.PlayerController|SetbShowMouseCursor (Game|GetPlayerController 0) false)))))

(fn ConstructionScript)